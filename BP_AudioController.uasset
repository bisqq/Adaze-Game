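; Audio visualizer controller that plays a sound and scales BP_Audio actors as equalizer bars.
; BeginPlay gathers those actors, insertion-sorts them by X position and starts playback.
; Tick samples a frequency spectrum slightly ahead of game time, which stands in for playback position, and cubes each band to set bar Z scale.
; An older tag-grouped polling version (SortEqualizer, SetIndexes, CalculateEqualizer) remains but is disconnected.
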(event EventBeginPlay
  (bind _equalizerobjectarray (Variables|Default|GetEqualizerObjectArray))
  (bind _audio (Variables|Default|GetAudio))
  (bind _outactors (Actor|GetAllActorsOfClass "/Game/MazeAudio/BP_Audio.BP_Audio_C"))
  (for _array_element _outactors
    (bind (_array_element_2 _array_index) (Utilities|Array|ForEachLoopwithBreak _equalizerobjectarray :!label _label)
      (:LoopBody
        (if (not (< (.X (Math|Vector|BreakVector (Transformation|GetActorLocation _array_element_2))) (.X (Math|Vector|BreakVector (Transformation|GetActorLocation _array_element)))))
          (goto _label Break)))
      (:Completed
        (Utilities|Array|Insert _equalizerobjectarray _array_element _array_index)
        (Audio|Components|Audio|SetSound _audio (Variables|Default|GetSound))
        (Audio|Components|Audio|Play _audio 0.0)))))

(event EventTick
  (params (DeltaSeconds :type Float%20%28single-precision%29))
  (bind _outspectrum (Class|SoundVisualizationStatics|CalculateFrequencySpectrum (Variables|Default|GetSound) 0 (+ (Utilities|Time|GetGameTimeinSeconds) 0.08) 0.19 24))
  (Variables|Default|SetFrequency%20Spectrum _outspectrum)
  (for (_array_element _array_index) (Variables|Default|GetEqualizerObjectArray)
    (Transformation|SetActorScale3D _array_element (Math|Vector|MakeVector 1.0 1.0 (+ (* (Math|Float|Clamp(Float) (/ (Utilities|Array|Get(acopy) (Variables|Default|GetFrequency%20Spectrum) _array_index) 2e+01) 0.0 5e+03) (Math|Float|Clamp(Float) (/ (Utilities|Array|Get(acopy) (Variables|Default|GetFrequency%20Spectrum) _array_index) 2e+01) 0.0 5e+03) (Math|Float|Clamp(Float) (/ (Utilities|Array|Get(acopy) (Variables|Default|GetFrequency%20Spectrum) _array_index) 2e+01) 0.0 5e+03)) 0.1)))))

(fn ConstructionScript)

(fn SortEqualizer
  (for _array_element (Variables|Default|GetEqualizerObjectArray)
    (if (Actor|ActorHasTag _array_element "EQ0")
      (Utilities|Array|Add (Variables|Default|GetEQ0) _array_element)
      (elif (Actor|ActorHasTag _array_element "EQ1")
        (Utilities|Array|Add (Variables|Default|GetEQ1) _array_element)
        (elif (Actor|ActorHasTag _array_element "EQ2")
          (Utilities|Array|Add (Variables|Default|GetEQ2) _array_element)
          (elif (Actor|ActorHasTag _array_element "EQ3")
            (Utilities|Array|Add (Variables|Default|GetEQ3) _array_element)
            (elif (Actor|ActorHasTag _array_element "EQ4")
              (Utilities|Array|Add (Variables|Default|GetEQ4) _array_element)
              (elif (Actor|ActorHasTag _array_element "EQ5")
                (Utilities|Array|Add (Variables|Default|GetEQ5) _array_element)
                (elif (Actor|ActorHasTag _array_element "EQ6")
                  (Utilities|Array|Add (Variables|Default|GetEQ6) _array_element)
                  (elif (Actor|ActorHasTag _array_element "EQ7")
                    (Utilities|Array|Add (Variables|Default|GetEQ7) _array_element)
                    (elif (Actor|ActorHasTag _array_element "EQ8")
                      (Utilities|Array|Add (Variables|Default|GetEQ8) _array_element)
                      (elif (Actor|ActorHasTag _array_element "EQ9")
                        (Utilities|Array|Add (Variables|Default|GetEQ9) _array_element)))))))))))))

(fn SetIndexes
  (bind _frequency_spectrum (Variables|Default|GetFrequency%20Spectrum))
  (bind _amplitude_array (Variables|Default|GetAmplitude%20Array))
  (Variables|Default|SetFreq0 (Utilities|Array|Get(acopy) _frequency_spectrum))
  (Variables|Default|SetFreq1 (Utilities|Array|Get(acopy) _frequency_spectrum 1))
  (Variables|Default|SetFreq2 (Utilities|Array|Get(acopy) _frequency_spectrum 2))
  (Variables|Default|SetFreq3 (Utilities|Array|Get(acopy) _frequency_spectrum 3))
  (Variables|Default|SetFreq4 (Utilities|Array|Get(acopy) _frequency_spectrum 4))
  (Variables|Default|SetFreq5 (Utilities|Array|Get(acopy) _frequency_spectrum 5))
  (Variables|Default|SetFreq6 (Utilities|Array|Get(acopy) _frequency_spectrum 6))
  (Variables|Default|SetFreq7 (Utilities|Array|Get(acopy) _frequency_spectrum 7))
  (Variables|Default|SetFreq8 (Utilities|Array|Get(acopy) _frequency_spectrum 8))
  (Variables|Default|SetFreq9 (Utilities|Array|Get(acopy) _frequency_spectrum 9))
  (Variables|Default|SetAmp0 (Utilities|Array|Get(acopy) _amplitude_array))
  (Variables|Default|SetAmp1 (Utilities|Array|Get(acopy) _amplitude_array 1))
  (Variables|Default|SetAmp2 (Utilities|Array|Get(acopy) _amplitude_array 2))
  (Variables|Default|SetAmp3 (Utilities|Array|Get(acopy) _amplitude_array 3))
  (Variables|Default|SetAmp4 (Utilities|Array|Get(acopy) _amplitude_array 4))
  (Variables|Default|SetAmp5 (Utilities|Array|Get(acopy) _amplitude_array 5))
  (Variables|Default|SetAmp6 (Utilities|Array|Get(acopy) _amplitude_array 6))
  (Variables|Default|SetAmp7 (Utilities|Array|Get(acopy) _amplitude_array 7))
  (Variables|Default|SetAmp8 (Utilities|Array|Get(acopy) _amplitude_array 8))
  (Variables|Default|SetAmp9 (Utilities|Array|Get(acopy) _amplitude_array 9)))

(fn CalculateEqualizer
  (for _array_element (Variables|Default|GetEQ0)
    (Transformation|SetActorTransform _array_element (Math|Transform|MakeTransform (.Location (Math|Transform|BreakTransform (Transformation|GetActorTransform _array_element))) (.Rotation (Math|Transform|BreakTransform (Transformation|GetActorTransform _array_element))) (+ (* (Math|Vector|ClampVectorSize (/ (Math|Vector|MakeVector (.X (Math|Vector|BreakVector (.Scale (Math|Transform|BreakTransform (Transformation|GetActorTransform _array_element))))) (.Y (Math|Vector|BreakVector (.Scale (Math|Transform|BreakTransform (Transformation|GetActorTransform _array_element))))) (Variables|Default|GetFreq0)) 2e+01) 0.0 5e+03) (Math|Vector|ClampVectorSize (/ (Math|Vector|MakeVector (.X (Math|Vector|BreakVector (.Scale (Math|Transform|BreakTransform (Transformation|GetActorTransform _array_element))))) (.Y (Math|Vector|BreakVector (.Scale (Math|Transform|BreakTransform (Transformation|GetActorTransform _array_element))))) (Variables|Default|GetFreq0)) 2e+01) 0.0 5e+03) (Math|Vector|ClampVectorSize (/ (Math|Vector|MakeVector (.X (Math|Vector|BreakVector (.Scale (Math|Transform|BreakTransform (Transformation|GetActorTransform _array_element))))) (.Y (Math|Vector|BreakVector (.Scale (Math|Transform|BreakTransform (Transformation|GetActorTransform _array_element))))) (Variables|Default|GetFreq0)) 2e+01) 0.0 5e+03)) 1.0))))
  (for _array_element_2 (Variables|Default|GetEQ1)
    (Transformation|SetActorTransform _array_element_2 (Math|Transform|MakeTransform (.Location (Math|Transform|BreakTransform (Transformation|GetActorTransform _array_element_2))) (.Rotation (Math|Transform|BreakTransform (Transformation|GetActorTransform _array_element_2))) (+ (* (Math|Vector|ClampVectorSize (/ (Math|Vector|MakeVector (.X (Math|Vector|BreakVector (.Scale (Math|Transform|BreakTransform (Transformation|GetActorTransform _array_element_2))))) (.Y (Math|Vector|BreakVector (.Scale (Math|Transform|BreakTransform (Transformation|GetActorTransform _array_element_2))))) (Variables|Default|GetFreq1)) 2e+01) 0.0 5e+03) (Math|Vector|ClampVectorSize (/ (Math|Vector|MakeVector (.X (Math|Vector|BreakVector (.Scale (Math|Transform|BreakTransform (Transformation|GetActorTransform _array_element_2))))) (.Y (Math|Vector|BreakVector (.Scale (Math|Transform|BreakTransform (Transformation|GetActorTransform _array_element_2))))) (Variables|Default|GetFreq1)) 2e+01) 0.0 5e+03) (Math|Vector|ClampVectorSize (/ (Math|Vector|MakeVector (.X (Math|Vector|BreakVector (.Scale (Math|Transform|BreakTransform (Transformation|GetActorTransform _array_element_2))))) (.Y (Math|Vector|BreakVector (.Scale (Math|Transform|BreakTransform (Transformation|GetActorTransform _array_element_2))))) (Variables|Default|GetFreq1)) 2e+01) 0.0 5e+03)) 1.0))))
  (for _array_element_3 (Variables|Default|GetEQ2)
    (Transformation|SetActorTransform _array_element_3 (Math|Transform|MakeTransform (.Location (Math|Transform|BreakTransform (Transformation|GetActorTransform _array_element_3))) (.Rotation (Math|Transform|BreakTransform (Transformation|GetActorTransform _array_element_3))) (+ (* (Math|Vector|ClampVectorSize (/ (Math|Vector|MakeVector (.X (Math|Vector|BreakVector (.Scale (Math|Transform|BreakTransform (Transformation|GetActorTransform _array_element_3))))) (.Y (Math|Vector|BreakVector (.Scale (Math|Transform|BreakTransform (Transformation|GetActorTransform _array_element_3))))) (Variables|Default|GetFreq2)) 2e+01) 0.0 5e+03) (Math|Vector|ClampVectorSize (/ (Math|Vector|MakeVector (.X (Math|Vector|BreakVector (.Scale (Math|Transform|BreakTransform (Transformation|GetActorTransform _array_element_3))))) (.Y (Math|Vector|BreakVector (.Scale (Math|Transform|BreakTransform (Transformation|GetActorTransform _array_element_3))))) (Variables|Default|GetFreq2)) 2e+01) 0.0 5e+03) (Math|Vector|ClampVectorSize (/ (Math|Vector|MakeVector (.X (Math|Vector|BreakVector (.Scale (Math|Transform|BreakTransform (Transformation|GetActorTransform _array_element_3))))) (.Y (Math|Vector|BreakVector (.Scale (Math|Transform|BreakTransform (Transformation|GetActorTransform _array_element_3))))) (Variables|Default|GetFreq2)) 2e+01) 0.0 5e+03)) 1.0))))
  (for _array_element_4 (Variables|Default|GetEQ3)
    (Transformation|SetActorTransform _array_element_4 (Math|Transform|MakeTransform (.Location (Math|Transform|BreakTransform (Transformation|GetActorTransform _array_element_4))) (.Rotation (Math|Transform|BreakTransform (Transformation|GetActorTransform _array_element_4))) (+ (* (Math|Vector|ClampVectorSize (/ (Math|Vector|MakeVector (.X (Math|Vector|BreakVector (.Scale (Math|Transform|BreakTransform (Transformation|GetActorTransform _array_element_4))))) (.Y (Math|Vector|BreakVector (.Scale (Math|Transform|BreakTransform (Transformation|GetActorTransform _array_element_4))))) (Variables|Default|GetFreq3)) 2e+01) 0.0 5e+03) (Math|Vector|ClampVectorSize (/ (Math|Vector|MakeVector (.X (Math|Vector|BreakVector (.Scale (Math|Transform|BreakTransform (Transformation|GetActorTransform _array_element_4))))) (.Y (Math|Vector|BreakVector (.Scale (Math|Transform|BreakTransform (Transformation|GetActorTransform _array_element_4))))) (Variables|Default|GetFreq3)) 2e+01) 0.0 5e+03) (Math|Vector|ClampVectorSize (/ (Math|Vector|MakeVector (.X (Math|Vector|BreakVector (.Scale (Math|Transform|BreakTransform (Transformation|GetActorTransform _array_element_4))))) (.Y (Math|Vector|BreakVector (.Scale (Math|Transform|BreakTransform (Transformation|GetActorTransform _array_element_4))))) (Variables|Default|GetFreq3)) 2e+01) 0.0 5e+03)) 1.0))))
  (for _array_element_5 (Variables|Default|GetEQ4)
    (Transformation|SetActorTransform _array_element_5 (Math|Transform|MakeTransform (.Location (Math|Transform|BreakTransform (Transformation|GetActorTransform _array_element_5))) (.Rotation (Math|Transform|BreakTransform (Transformation|GetActorTransform _array_element_5))) (+ (* (Math|Vector|ClampVectorSize (/ (Math|Vector|MakeVector (.X (Math|Vector|BreakVector (.Scale (Math|Transform|BreakTransform (Transformation|GetActorTransform _array_element_5))))) (.Y (Math|Vector|BreakVector (.Scale (Math|Transform|BreakTransform (Transformation|GetActorTransform _array_element_5))))) (Variables|Default|GetFreq4)) 2e+01) 0.0 5e+03) (Math|Vector|ClampVectorSize (/ (Math|Vector|MakeVector (.X (Math|Vector|BreakVector (.Scale (Math|Transform|BreakTransform (Transformation|GetActorTransform _array_element_5))))) (.Y (Math|Vector|BreakVector (.Scale (Math|Transform|BreakTransform (Transformation|GetActorTransform _array_element_5))))) (Variables|Default|GetFreq4)) 2e+01) 0.0 5e+03) (Math|Vector|ClampVectorSize (/ (Math|Vector|MakeVector (.X (Math|Vector|BreakVector (.Scale (Math|Transform|BreakTransform (Transformation|GetActorTransform _array_element_5))))) (.Y (Math|Vector|BreakVector (.Scale (Math|Transform|BreakTransform (Transformation|GetActorTransform _array_element_5))))) (Variables|Default|GetFreq4)) 2e+01) 0.0 5e+03)) 1.0))))
  (for _array_element_6 (Variables|Default|GetEQ5)
    (Transformation|SetActorTransform _array_element_6 (Math|Transform|MakeTransform (.Location (Math|Transform|BreakTransform (Transformation|GetActorTransform _array_element_6))) (.Rotation (Math|Transform|BreakTransform (Transformation|GetActorTransform _array_element_6))) (+ (* (Math|Vector|ClampVectorSize (/ (Math|Vector|MakeVector (.X (Math|Vector|BreakVector (.Scale (Math|Transform|BreakTransform (Transformation|GetActorTransform _array_element_6))))) (.Y (Math|Vector|BreakVector (.Scale (Math|Transform|BreakTransform (Transformation|GetActorTransform _array_element_6))))) (Variables|Default|GetFreq5)) 2e+01) 0.0 5e+03) (Math|Vector|ClampVectorSize (/ (Math|Vector|MakeVector (.X (Math|Vector|BreakVector (.Scale (Math|Transform|BreakTransform (Transformation|GetActorTransform _array_element_6))))) (.Y (Math|Vector|BreakVector (.Scale (Math|Transform|BreakTransform (Transformation|GetActorTransform _array_element_6))))) (Variables|Default|GetFreq5)) 2e+01) 0.0 5e+03) (Math|Vector|ClampVectorSize (/ (Math|Vector|MakeVector (.X (Math|Vector|BreakVector (.Scale (Math|Transform|BreakTransform (Transformation|GetActorTransform _array_element_6))))) (.Y (Math|Vector|BreakVector (.Scale (Math|Transform|BreakTransform (Transformation|GetActorTransform _array_element_6))))) (Variables|Default|GetFreq5)) 2e+01) 0.0 5e+03)) 1.0)))))